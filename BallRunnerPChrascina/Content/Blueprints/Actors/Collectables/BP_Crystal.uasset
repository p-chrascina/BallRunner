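; BP_Crystal is a collectable crystal actor that spins around its yaw axis every tick.
; When a pawn overlaps its sphere, it caches its location, scale and light intensity, then plays a timeline.
; The timeline's separate curves lerp it toward player 0's current position, shrink it to zero and fade its point light.
; The actor destroys itself when the timeline finishes.
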(event OnComponentBeginOverlap(Sphere)
  (params (OverlappedComponent :type Primitive%20Component%20Object%20Reference) (OtherActor :type Actor%20Object%20Reference) (OtherComp :type Primitive%20Component%20Object%20Reference) (OtherBodyIndex :type Integer) (bFromSweep :type Boolean) (SweepResult :type Hit%20Result%20Structure%20%28by%20ref%29))
  (Utilities|IsPawn OtherActor
    (:True
      (CallFunction|SetStartValues)
      (bind (_direction _locationintime _scaleintime _lightintime) (Timeline|TimelineCrystal Play)
        (:Update
          (CallFunction|ChangeCrystalLocation _locationintime)
          (CallFunction|ChangeCrystalScale _scaleintime)
          (Rendering|Components|Light|SetIntensity (Variables|Default|GetPointLight) (Math|Float|Lerp (Variables|Default|GetLerpStartLight) 0.0 _lightintime)))
        (:Finished
          (Actor|DestroyActor))))))

(event EventBeginPlay)

(event Collision|EventActorBeginOverlap
  (params (OtherActor :type Actor%20Object%20Reference)))

(event EventTick
  (params (DeltaSeconds :type Float%20%28single-precision%29))
  (Transformation|AddActorLocalRotation (Math|Rotator|MakeRotator 0.0 0.0 (* DeltaSeconds (Variables|Default|GetRotation))) false false))

(fn ConstructionScript)

(fn ChangeCrystalLocation
  (params (Alpha :type Float%20%28single-precision%29))
  (Transformation|SetActorLocation (Math|Vector|Lerp(Vector) (Variables|Default|GetLerpStartLocation) (Transformation|GetActorLocation (Game|Player|GetPlayerPawn 0)) Alpha) false false))

(fn SetStartValues
  (Variables|Default|SetLerpStartLocation (Transformation|GetActorLocation))
  (Variables|Default|SetLerpStartScale (Transformation|GetActorScale3D))
  (Variables|Default|SetLerpStartLight (Variables|/Script/Engine.LightComponentBase|GetIntensity (Variables|Default|GetPointLight))))

(fn ChangeCrystalScale
  (params (Alpha :type Float%20%28single-precision%29))
  (Transformation|SetActorScale3D (Math|Vector|Lerp(Vector) (Variables|Default|GetLerpStartScale) "0, 0, 0" Alpha)))