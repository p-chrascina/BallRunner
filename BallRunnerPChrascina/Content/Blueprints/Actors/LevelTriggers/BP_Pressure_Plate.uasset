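; BP_Pressure_Plate is a level trigger that opens its matching BP_Door when a pawn steps on it.
; Sphere overlap restarts the Pressure timeline, which drives the Cylinder's relative X location.
; On every timeline update it searches all BP_Door actors for a DoorID equal to PlateID, calls Open and turns the point light green.
; There is no end-overlap handling.
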(event OnComponentBeginOverlap(Sphere)
  (params (OverlappedComponent :type Primitive%20Component%20Object%20Reference) (OtherActor :type Actor%20Object%20Reference) (OtherComp :type Primitive%20Component%20Object%20Reference) (OtherBodyIndex :type Integer) (bFromSweep :type Boolean) (SweepResult :type Hit%20Result%20Structure%20%28by%20ref%29))
  (Utilities|IsPawn OtherActor
    (:True
      (bind _platelocationx (Timeline|Pressure PlayFromStart)
        (:Update
          (Transformation|SetRelativeLocation (Variables|Default|GetCylinder) (Math|Vector|MakeVector _platelocationx 0.0 0.0) false false)
          (bind _outactors (Actor|GetAllActorsOfClass "/Game/Blueprints/Actors/LevelTriggers/BP_Door.BP_Door_C"))
          (for _array_element _outactors
            (if (== (Variables|/Game/Blueprints/Actors/LevelTriggers/BP_Door.BP_Door_C|GetDoorID _array_element) (Variables|Default|GetPlateID))
              (Variables|Default|SetDoor _array_element)))
          (Utilities|IsValid (Variables|Default|GetDoor)
            (:Is%20Valid
              (Default|Open (Variables|Default|GetDoor))
              (Rendering|Components|Light|SetLightColor (Variables|Default|GetPointLight) "(R=0.000000,G=1.000000,B=0.650417,A=1.000000)" true))))))))

(fn ConstructionScript)