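; Player pawn that rolls a physics ball from forward/back and left/right axis input.
; Each axis applies mass-independent torque (acceleration change) to the Ball, scaled by a Multiply variable, with the forward/back torque negated.
; The camera fades in on BeginPlay.
; Any damage acts as death, fading the camera out and reloading the current level after a short delay.
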(event EventBeginPlay
  (CameraFades|StartCameraFade :self (Game|GetPlayerCameraManager 0) :FromAlpha 1.0 :Duration 2.0))

(event Game|Damage|EventAnyDamage
  (params (Damage :type Float%20%28single-precision%29) (DamageType :type Damage%20Type%20Object%20Reference) (InstigatedBy :type Controller%20Object%20Reference) (DamageCauser :type Actor%20Object%20Reference))
  (bind _returnvalue (Math|Float|MakeLiteralFloat 1.0))
  (CameraFades|StartCameraFade :self (Game|GetPlayerCameraManager 0) :ToAlpha 1.0 :Duration _returnvalue)
  (Utilities|FlowControl|Delay _returnvalue)
  (bind _returnvalue_2 (Game|GetCurrentLevelName true))
  (Game|OpenLevel(byName) (Utilities|String|StringToName _returnvalue_2)))

(event Input|AxisEvents|InputAxisMove_Forward/Back
  (params (AxisValue :type Float%20%28single-precision%29))
  (CallFunction|TorqueX AxisValue))

(event Input|AxisEvents|InputAxisMove_Left/Right
  (params (AxisValue :type Float%20%28single-precision%29))
  (CallFunction|TorqueY AxisValue))

(fn ConstructionScript)

(fn TorqueY
  (params (A :type Float%20%28single-precision%29))
  (Class|PrimitiveComponent|AddTorqueinRadians (Variables|Default|GetBall) (Math|Vector|MakeVector 0.0 (* A (Variables|Default|GetMultiply)) 0.0) "None" true))

(fn TorqueX
  (params (A :type Float%20%28single-precision%29))
  (Class|PrimitiveComponent|AddTorqueinRadians (Variables|Default|GetBall) (Math|Vector|MakeVector (* (* A (Variables|Default|GetMultiply)) -1.0) 0.0 0.0) "None" true))