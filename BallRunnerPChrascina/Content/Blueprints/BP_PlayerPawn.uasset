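; Player pawn that moves by rolling its Ball component with physics torque.
; Forward/back and left/right axis inputs apply torque around X (negated) and Y, scaled by the Multiply variable.
; Torque is applied as an acceleration change, so the ball's mass does not affect it.
; BeginPlay fades the player camera in over two seconds.
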(event EventBeginPlay
  (CameraFades|StartCameraFade :self (Game|GetPlayerCameraManager 0) :FromAlpha 1.0 :ToAlpha 0.0 :Duration 2.0))

(event Input|AxisEvents|InputAxisMove_Forward/Back
  (params (AxisValue :type Float%20%28single-precision%29))
  (Class|PrimitiveComponent|AddTorqueinRadians (Variables|Default|GetBall) (Math|Vector|MakeVector (* (* AxisValue (Variables|Default|GetMultiply)) -1.0) 0.0 0.0) "None" true))

(event Input|AxisEvents|InputAxisMove_Left/Right
  (params (AxisValue :type Float%20%28single-precision%29))
  (Class|PrimitiveComponent|AddTorqueinRadians (Variables|Default|GetBall) (Math|Vector|MakeVector 0.0 (* AxisValue (Variables|Default|GetMultiply)) 0.0) "None" true))

(fn ConstructionScript)